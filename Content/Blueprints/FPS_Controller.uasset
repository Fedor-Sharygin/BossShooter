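; First-person character controller Blueprint handling movement, mouse look, jumping and dashing.
; Movement follows the control rotation's yaw only, while look input is scaled by mouse sensitivity relative to its maximum.
; Dash launches the character along the combined movement input, falling back to facing direction without input, using DashPulse on the ground and a fixed strength otherwise.
; Jump triggers only while grounded.
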(event `InputAction|Dash`
  (params (Key :type "Key Structure"))
  (bind _returnvalue (`KismetMathLibrary.MakeRotator` 0.0 0.0 (.yaw (`self.GetControlRotation`))))
  (bind _returnvalue_2 (`KismetMathLibrary.GetForwardVector` _returnvalue))
  ;[1 1 1] Movement
  ;;[1 1 1] Dashing
  (:`Pressed`
    (bind _returnvalue_3 (`KismetMathLibrary.Normal` (+ (* _returnvalue_2 (stale `InputAxis|MoveForward` AxisValue)) (* (`KismetMathLibrary.GetRightVector` _returnvalue) (stale `InputAxis|MoveRight` AxisValue)))))
    (`self.LaunchCharacter` (* (`KismetMathLibrary.SelectVector` _returnvalue_3 _returnvalue_2 (not (`KismetMathLibrary.Vector_IsZero` _returnvalue_3))) (`KismetMathLibrary.SelectFloat` (`self.DashPulse`) 600.0 (`NavMovementComponent.IsMovingOnGround` (`self.CharacterMovement`)))))))

(event `InputAxis|MoveForward`
  (params (AxisValue :type "Float (single-precision)"))
  ;[1 1 1] Movement
  ;;[1 1 1] Directional Movement
  (`self.AddMovementInput` (* (`KismetMathLibrary.GetForwardVector` (`KismetMathLibrary.MakeRotator` 0.0 0.0 (.yaw (`self.GetControlRotation`)))) AxisValue)))

(event `InputAxis|MoveRight`
  (params (AxisValue :type "Float (single-precision)"))
  ;[1 1 1] Movement
  ;;[1 1 1] Directional Movement
  (`self.AddMovementInput` (* (`KismetMathLibrary.GetRightVector` (`KismetMathLibrary.MakeRotator` 0.0 0.0 (.yaw (`self.GetControlRotation`)))) AxisValue)))

(event `InputAction|Jump`
  (params (Key :type "Key Structure"))
  ;[1 1 1] Movement
  ;;[1 1 1] Jumping
  (:`Pressed`
    (if (`NavMovementComponent.IsMovingOnGround` (`self.CharacterMovement`))
      (`self.Jump`))))

(event `InputAxis|LookUp`
  (params (AxisValue :type "Float (single-precision)"))
  ;[1 1 1] Look Around
  (`self.AddControllerPitchInput` (* AxisValue (/ (`self.MouseSensitivity`) (`self.MaxMSens`)))))

(event `InputAxis|Turn`
  (params (AxisValue :type "Float (single-precision)"))
  ;[1 1 1] Look Around
  (`self.AddControllerYawInput` (* AxisValue (/ (`self.MouseSensitivity`) (`self.MaxMSens`)))))

(fn `UserConstructionScript`)